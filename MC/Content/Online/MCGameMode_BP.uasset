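; Online game mode that manages the lifetime of world chunks around the player.
; SpawnChunkEvent spawns a Chunks_BP actor at a given location and records it in the AllChunks map by chunk index, skipping indices already present.
; Every tick, RemoveChunks destroys and unregisters chunks farther from PlayerChunkIndex than ChunkRange plus a small margin.
; An unused collapsed graph holds an alternative range-based grid spawning loop.
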(event EventBeginPlay
  (Variables|Default|SetPawn (Game|Player|GetPlayerPawn 0)))

(event EventTick
  (params (DeltaSeconds :type Float%20%28single-precision%29))
  (CallFunction|RemoveChunks))

(event EventSpawnChunkEvent
  (params (ToSpawn :type Object%20Class%20Reference) (Location :type Vector%20%28by%20ref%29 :default "0, 0, 0") (ChunkIndex :type Vector%202D%20Structure))
  (if (not (.ReturnValue (Utilities|Map|Find (Variables|Default|GetAllChunks) ChunkIndex)))
    (bind _returnvalue (Game|SpawnActorfromClass "/Game/BluePrint/Chunks_BP.Chunks_BP_C" (Math|Transform|MakeTransform Location "0, 0, 0" "1,1,1") "Undefined" 0 0))
    (Utilities|Map|Add (Variables|Default|GetAllChunks) ChunkIndex _returnvalue)))

(fn ConstructionScript)

(fn RemoveChunks
  (bind _allchunks (Variables|Default|GetAllChunks))
  (bind _keys (Utilities|Map|Keys (Variables|Default|GetAllChunks)))
  (for _array_element _keys
    (if (> (Math|Vector|Distance2D(Vector) _array_element (Variables|Default|GetPlayerChunkIndex)) (Math|Conversions|ToFloat(Integer) (+ (Variables|Default|GetChunkRange) 2)))
      (Actor|DestroyActor (.Value (Utilities|Map|Find _allchunks _array_element)))
      (Utilities|Map|Remove _allchunks _array_element))))